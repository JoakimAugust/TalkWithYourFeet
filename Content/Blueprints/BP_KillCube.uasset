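; BP_KillCube is a damageable cube actor with a health bar widget that turns toward the player.
; ActorDamage lowers Health by DamageAmount, and UpdateHealth calls ActorDeath to destroy the actor at zero or below.
; Tick runs UpdateHealth and the bar update only while Health is above zero, so that death check cannot pass from Tick.
; The bar update sets progress on a 100-point scale and rotates the widget with FindLookAtRotation.
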(event Custom|Actor%20Death
  ;[1 1 1] Health System
  (Actor|DestroyActor))

(event Custom|UpdateHealth
  ;[1 1 1] Health System
  (if (<= (Variables|Default|Gethealth) 0.0)
    (CallFunction|ActorDeath)))

(event Custom|UpdateHealtbar
  (bind _healthbar (Variables|Default|GetHealthBar))
  ;[1 1 1] Health Bar percent and rotation
  (bind _asbpw_kill_cube_health_bar (Utilities|Casting|CastToBPW_KillCubeHealthBar (UserInterface|GetUserWidgetObject (Variables|Default|GetHealthBar))))
  (Progress|SetPercent (Variables|/Game/Blueprints/BPW_KillCubeHealthBar.BPW_KillCubeHealthBar_C|GetProgressBar_93 _asbpw_kill_cube_health_bar) (/ (Variables|Default|Gethealth) 1e+02))
  (Transformation|SetWorldRotation _healthbar (Math|Rotator|FindLookatRotation (Transformation|GetWorldLocation _healthbar) (Transformation|GetActorLocation (Game|GetPlayerCharacter 0))) false false))

(event Custom|Actor%20Damage
  (params (Damage :type Float%20%28single-precision%29))
  ;[1 1 1] Health System
  (Variables|Default|Sethealth (- (Variables|Default|Gethealth) (Variables|Default|GetDamage%20Amount))))

(event EventTick
  (params (DeltaSeconds :type Float%20%28single-precision%29))
  ;[1 1 1] Event Tick
  (if (> (Variables|Default|Gethealth) 0.0)
    (Utilities|FlowControl|Sequence
      (:then_0
        (CallFunction|UpdateHealth))
      (:then_1
        (CallFunction|UpdateHealtbar)))))

(fn ConstructionScript)