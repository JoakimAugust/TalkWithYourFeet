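; Game mode for a multiplayer Red versus Green zone-capture match with a countdown timer.
; Once all players join, it gathers their info, splits teams, spawns characters at tagged PlayerStarts and starts the timer when all are spawned.
; Each tick, captured zones raise team percentages, and score bars and per-team ComSys states are pushed to player controllers.
; A full percentage or expired timer shows the winner, then destroys sessions after a delay.
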(event Custom|UpdateTimer
  ;[1 1 1] Start timer
  (if (Variables|Default|GetMachIsPlaying)
    (if (and (<= (Variables|Default|GetMinutes) 0) (<= (Variables|Default|GetSeconds) 0))
      (CallFunction|EndGame)
      (else
        (if (> (Variables|Default|GetSeconds) 0)
          (Math|Integer|DecrementInt (Variables|Default|GetSeconds)
            (:%20%20
              _))
          (else
            (Math|Integer|DecrementInt (Variables|Default|GetMinutes)
              (:%20%20
                (Variables|Default|SetSeconds 59)))))
        (for _array_element (Variables|Default|GetAllPlayers)
          (bind _asbp_gameplay_pc (Utilities|Casting|CastToBP_GameplayPC _array_element))
          (Default|UpdateTimer _asbp_gameplay_pc (Variables|Default|GetMinutes) (Variables|Default|GetSeconds)))))))

(event Custom|UpdateComSysUnit
  (params (PlayerTeam :type Enum_PlayerTeam%20Enum) (ComSysIndex :type Integer) (ComSysState :type Enum_ComSysState%20Enum) (TaggedActor :type Actor%20Object%20Reference))
  ;[1 1 1] Update ComSys
  (switch Utilities|FlowControl|Switch|SwitchonEnum_PlayerTeam PlayerTeam
    (:NewEnumerator0
      (Utilities|Struct|SetmembersinStruct_ComSysUnit (Utilities|Array|Get(acopy) (Variables|ComSys|GetRedComSys) ComSysIndex) ComSysState TaggedActor))
    (:NewEnumerator1
      (Utilities|Struct|SetmembersinStruct_ComSysUnit (Utilities|Array|Get(acopy) (Variables|ComSys|GetGreenComSys) ComSysIndex) ComSysState TaggedActor))))

(event Custom|EndGame
  ;[1 1 1] End game
  (Variables|Default|SetMachIsPlaying false)
  (bind _text (CallFunction|GetWinnerText))
  (for _array_element (Variables|Default|GetAllPlayers)
    (bind _asbp_gameplay_pc (Utilities|Casting|CastToBP_GameplayPC _array_element))
    (Default|ShowWinnerText _asbp_gameplay_pc _text))
  (Utilities|FlowControl|Delay 5.0)
  (for _array_element_2 (Variables|Default|GetAllPlayers)
    (Default|DestroySessionforPlayer (.AsBP%20Gameplay%20PC (Utilities|Casting|CastToBP_GameplayPC _array_element_2)))))

(event Custom|Start%20Timer
  ;[1 1 1] Start timer
  (Utilities|Time|SetTimerbyEvent (delegate Custom|UpdateTimer) 1.0 true))

(event Custom|PossessAllPlayers
  ;[1 1 1] Respawn all players and start timer
  (for _array_element (Variables|Default|GetAllPlayers)
    (Pawn|Possess (.AsBP%20Gameplay%20PC (Utilities|Casting|CastToBP_GameplayPC _array_element)) (Variables|/Game/Blueprints/Gameplay/BP_GameplayPC.BP_GameplayPC_C|GetPlayerCharacterRef (.AsBP%20Gameplay%20PC (Utilities|Casting|CastToBP_GameplayPC _array_element))))
    (Input|EnableInput (Variables|/Game/Blueprints/Gameplay/BP_GameplayPC.BP_GameplayPC_C|GetPlayerCharacterRef (.AsBP%20Gameplay%20PC (Utilities|Casting|CastToBP_GameplayPC _array_element))) (.AsBP%20Gameplay%20PC (Utilities|Casting|CastToBP_GameplayPC _array_element))))
  (CallFunction|StartTimer))

(event Custom|UpdateComSysForPlayers
  ;[1 1 1] Update ComSys
  (for _array_element (Variables|ComSys|GetRedPlayers)
    (Utilities|UpdateComSysRedPlayer _array_element))
  (for _array_element_2 (Variables|ComSys|GetGreenPlayers)
    (Utilities|UpdateComSysGreenPlayer _array_element_2)))

(event Custom|RespawnPlayer
  (params (Controller :type Player%20Controller%20Object%20Reference) (PlayerInfo :type Struct%20Player%20Info%20Structure))
  (bind _returnvalue (Pawn|GetControlledPawn Controller))
  ;[1 1 1] Respawn player
  (Utilities|IsValid _returnvalue
    (:Is%20Valid
      (Actor|DestroyActor _returnvalue))
    (:Is%20Not%20Valid
      _))
  (CallFunction|RespawnPlayerFunc Controller PlayerInfo))

(event Custom|AddPlayerInfo
  (params (PlayerInfo :type Struct%20Player%20Info%20Structure) (Index :type Integer))
  ;[1 1 1] Add player info to server, called from client
  (Utilities|Array|SetArrayElem (Variables|Default|GetAllPlayerInfo) Index PlayerInfo)
  (bind _result (Math|Integer|IncrementInt (Variables|Default|GetAddedPlayerInfo))
    (:%20%20
      (if (== _result (Variables|/Game/Blueprints/General/BP_GameInstance.BP_GameInstance_C|GetMaxPlayers (Variables|Default|GetGameInstanceRef)))
        (CallFunction|SplitPlayersinTeams)))))

(event Custom|SplitPlayersInTeams
  ;[1 1 1] Split player in teams
  (for (_array_element _array_index) (Variables|Default|GetAllPlayers)
    (if (Utilities|Enum|Equal(Enum) (.Team (Utilities|Struct|BreakStruct_PlayerInfo (Utilities|Array|Get(acopy) (Variables|Default|GetAllPlayerInfo) _array_index))) "NewEnumerator0")
      (bind _returnvalue (Utilities|Array|Add (Variables|ComSys|GetRedPlayers) (.AsBP%20Gameplay%20PC (Utilities|Casting|CastToBP_GameplayPC _array_element))))
      (Default|SetComSysIndexinClient (.AsBP%20Gameplay%20PC (Utilities|Casting|CastToBP_GameplayPC _array_element)) _returnvalue)))
  (for (_array_element_2 _array_index_2) (Variables|Default|GetAllPlayers)
    (if (Utilities|Enum|Equal(Enum) (.Team (Utilities|Struct|BreakStruct_PlayerInfo (Utilities|Array|Get(acopy) (Variables|Default|GetAllPlayerInfo) _array_index_2))) "NewEnumerator1")
      (bind _returnvalue_2 (Utilities|Array|Add (Variables|ComSys|GetGreenPlayers) (.AsBP%20Gameplay%20PC (Utilities|Casting|CastToBP_GameplayPC _array_element_2))))
      (Default|SetComSysIndexinClient (.AsBP%20Gameplay%20PC (Utilities|Casting|CastToBP_GameplayPC _array_element_2)) _returnvalue_2)))
  (CallFunction|SpawnAllPlayers))

(event Custom|SpawnAllPlayers
  ;[1 1 1] Respawn all players and start timer
  (for _array_element (Variables|Default|GetAllPlayers)
    (Default|CallRespawnPlayer (.AsBP%20Gameplay%20PC (Utilities|Casting|CastToBP_GameplayPC _array_element)))))

(event Custom|UpdateTeamPercent
  ;[1 1 1] Updating of team percent
  (for _array_element (Variables|Default|GetZones)
    (if (> (Variables|/Game/Blueprints/Gameplay/Zone/PB_Zone.PB_Zone_C|GetRedProgress _array_element) 0.9)
      (bind _output_get (Variables|Default|SetRedPercent (+ (Variables|Default|GetRedPercent) (/ 0.01 (Variables|Default|GetFramesPerPercent)))))
      (if (or (>= _output_get 1.0) (>= (stale _output_get_2) 1.0)) :!label _label
        (CallFunction|EndGame))
      (elif (> (Variables|/Game/Blueprints/Gameplay/Zone/PB_Zone.PB_Zone_C|GetGreenProgress _array_element) 0.9)
        (bind _output_get_2 (Variables|Default|SetGreenPercent (+ (Variables|Default|GetGreenPercent) (/ 0.01 (Variables|Default|GetFramesPerPercent)))))
        (goto _label)))))

(event Custom|GetAllPlayerInfo
  ;[1 1 1] Get all connected player info
  (for (_array_element _array_index) (Variables|Default|GetAllPlayers)
    (Default|CallSendInfotoServer (.AsBP%20Gameplay%20PC (Utilities|Casting|CastToBP_GameplayPC _array_element)) _array_index)))

(event EventOnLogout
  (params (ExitingController :type Controller%20Object%20Reference))
  ;[1 1 1] Destroy session caller
  (bind _asbp_gameplay_pc (Utilities|Casting|CastToBP_GameplayPC ExitingController))
  (Default|CallDestroySession (Variables|Default|GetGameInstanceRef) _asbp_gameplay_pc))

(event EventTick
  (params (DeltaSeconds :type Float%20%28single-precision%29))
  ;[1 1 1] Frame update
  (if (Variables|Default|GetMachIsPlaying)
    (CallFunction|UpdateTeamPercent)
    (for _array_element (Variables|Default|GetAllPlayers)
      (bind _asbp_gameplay_pc (Utilities|Casting|CastToBP_GameplayPC _array_element))
      (Default|UpdateTeamBars _asbp_gameplay_pc (Variables|Default|GetRedPercent) (Variables|Default|GetGreenPercent))
      (CallFunction|UpdateComSysforPlayers))))

(event EventPostLogin
  (params (NewPlayer :type Player%20Controller%20Object%20Reference))
  ;[1 1 1] Set up player on login
  (Default|PlayerSetup (.AsBP%20Gameplay%20PC (Utilities|Casting|CastToBP_GameplayPC NewPlayer)))
  (Networking|SwitchHasAuthority
    (:Authority
      (bind _returnvalue (Utilities|Array|Add (Variables|Default|GetAllPlayers) NewPlayer))
      (if (== _returnvalue (|GetMaxPlayers-1_2_2))
        (CallFunction|GetAllPlayerInfo)))))

(fn ConstructionScript
  (bind _asbp_game_instance (Utilities|Casting|CastToBP_GameInstance (Game|GetGameInstance)))
  (Variables|Default|SetGameInstanceRef _asbp_game_instance)
  (Networking|SwitchHasAuthority
    (:Authority
      (Variables|Default|SetMaxPlayers (Variables|/Game/Blueprints/General/BP_GameInstance.BP_GameInstance_C|GetMaxPlayers (Variables|Default|GetGameInstanceRef)))
      (bind _outactors (Actor|GetAllActorsOfClass "/Game/Blueprints/Gameplay/Zone/PB_Zone.PB_Zone_C"))
      (Variables|Default|SetZones _outactors))))

(fn RespawnPlayerFunc
  (params (PlayerController :type Player%20Controller%20Object%20Reference) (PlayerInfo :type Struct%20Player%20Info%20Structure))
  (bind (_returnvalue _spawncollisionhandlingmethod) (|GetSpawnPointLocationAndCollisionHandle_2))
  (bind (_returnvalue_2 _spawncollisionhandlingmethod_2) (|GetSpawnPointLocationAndCollisionHandle))
  (bind _asbp_gameplay_pc (Utilities|Casting|CastToBP_GameplayPC PlayerController))
  (LocalVariables|SetPlayerControllerRef _asbp_gameplay_pc)
  (LocalVariables|SetPlayerInfoVar PlayerInfo)
  (Utilities|IsValid (Variables|/Game/Blueprints/Gameplay/BP_GameplayPC.BP_GameplayPC_C|GetPlayerStart (LocalVariables|GetPlayerControllerRef))
    (:Is%20Valid
      (LocalVariables|SetSpawnPoint (Variables|/Game/Blueprints/Gameplay/BP_GameplayPC.BP_GameplayPC_C|GetPlayerStart (LocalVariables|GetPlayerControllerRef)))
      (bind _returnvalue_3 (Game|SpawnActorfromClass (Game|GetPlayerCharacter) _returnvalue_2 _spawncollisionhandlingmethod_2 0 0))
      (bind _output_get (Variables|/Game/Blueprints/Gameplay/BP_GameplayPC.BP_GameplayPC_C|SetPlayerCharacterRef (LocalVariables|GetPlayerControllerRef) _returnvalue_3))
      (Pawn|Possess (LocalVariables|GetPlayerControllerRef) _returnvalue_3)
      (Input|EnableInput _output_get (LocalVariables|GetPlayerControllerRef)))
    (:Is%20Not%20Valid
      (switch Utilities|FlowControl|Switch|SwitchonEnum_PlayerTeam (.Team (Utilities|Struct|BreakStruct_PlayerInfo (LocalVariables|GetPlayerInfoVar)))
        (:NewEnumerator2
          (LocalVariables|SetSearchTag "RED" :!label _label))
        (:NewEnumerator0
          (goto _label))
        (:NewEnumerator1
          (LocalVariables|SetSearchTag "GREEN")))
      (bind _outactors (Actor|GetAllActorsOfClass "/Script/Engine.PlayerStart"))
      (bind _array_element (Utilities|Array|ForEachLoopwithBreak _outactors :!label _label_2)
        (:LoopBody
          (if (Utilities|Name|Equal(Name) (Variables|/Script/Engine.PlayerStart|GetPlayerStartTag _array_element) (LocalVariables|GetSearchTag))
            (Variables|/Script/Engine.PlayerStart|SetPlayerStartTag _array_element "TAKEN")
            (bind _output_get_2 (Variables|/Game/Blueprints/Gameplay/BP_GameplayPC.BP_GameplayPC_C|SetPlayerStart (LocalVariables|GetPlayerControllerRef) _array_element))
            (LocalVariables|SetSpawnPoint _output_get_2)
            (goto _label_2 Break)))
        (:Completed
          (bind _returnvalue_4 (Game|SpawnActorfromClass (|GetPlayerCharacter_2) _returnvalue _spawncollisionhandlingmethod 0 0))
          (Variables|/Game/Blueprints/Gameplay/BP_GameplayPC.BP_GameplayPC_C|SetPlayerCharacterRef (LocalVariables|GetPlayerControllerRef) _returnvalue_4)
          (bind _result (Math|Integer|IncrementInt (Variables|Default|GetSpawnedPlayerCharacters))
            (:%20%20
              (if (== _result (Variables|Default|GetMaxPlayers))
                (CallFunction|PossessAllPlayers)))))))))

(fn GetWinnerText
  (if (> (Variables|Default|GetRedPercent) (Variables|Default|GetGreenPercent))
    (LocalVariables|SetMessage "Red team winns!")
    (elif (< (Variables|Default|GetRedPercent) (Variables|Default|GetGreenPercent))
      (LocalVariables|SetMessage "Green team winns!")
      (else
        (LocalVariables|SetMessage "It's a draw!"))))
  (return (LocalVariables|GetMessage)))

(fn GetComSysState
  (params (PlayerTeam :type Enum_PlayerTeam%20Enum) (ComSysIndex :type Integer))
  (switch Utilities|FlowControl|Switch|SwitchonEnum_PlayerTeam PlayerTeam
    (:NewEnumerator0
      (return (.State (Utilities|Struct|BreakStruct_ComSysUnit (Utilities|Array|Get(acopy) (Variables|ComSys|GetRedComSys) ComSysIndex)))))
    (:NewEnumerator1
      (return (.State (Utilities|Struct|BreakStruct_ComSysUnit (Utilities|Array|Get(acopy) (Variables|ComSys|GetGreenComSys) ComSysIndex)))))))