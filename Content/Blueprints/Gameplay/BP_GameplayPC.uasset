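; Gameplay player controller for a Red vs Green team match, forwarding attack and run input to the team's character.
; ComSys inputs toggle attack, defend, follow or heal callouts, using forward sphere traces to tag enemies or zones, otherwise the player's own character.
; Callouts, player info and respawns route to BP_GameplayGM, while update events drive HUD markers, timer and team bars.
; It also tracks health with a damage cooldown, respawning at zero.
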(event Custom|SendInfoToServer
  (params (PlayerInfo :type Struct%20Player%20Info%20Structure) (Index :type Integer))
  ;[1 1 1] Server stuff
  (Default|AddPlayerInfo (Variables|Default|GetGameModeRef) PlayerInfo Index))

(event Custom|PlayerSetup
  ;[1 1 1] Initial player setup
  (bind _asbp_hud (Utilities|Casting|CastToBP_HUD (HUD|GetHUD)))
  (Variables|Default|SetHudRef _asbp_hud)
  (bind _asbp_game_instance (Utilities|Casting|CastToBP_GameInstance (Game|GetGameInstance)))
  (Variables|PlayerData|SetPlayerInfo (Variables|/Game/Blueprints/General/BP_GameInstance.BP_GameInstance_C|GetPlayerInfo _asbp_game_instance)))

(event Custom|ShowWinnerText
  (params (Text :type String))
  ;[1 1 1] Print winner text
  (Development|PrintString Text))

(event Custom|CallSendInfoToServer
  (params (Index :type Integer))
  ;[1 1 1] Server stuff
  (CallFunction|SendInfotoServer (Variables|PlayerData|GetPlayerInfo) Index))

(event Custom|Update%20timer
  (params (Minutes :type Integer) (Seconds :type Integer))
  ;[1 1 1] Update timer for player
  (Default|SetTime (Variables|/Game/Blueprints/Gameplay/HUD/BP_HUD.BP_HUD_C|GetMatchBar (Variables|Default|GetHudRef)) Minutes Seconds))

(event Custom|PlayerRespawnServerLink
  (params (PlayerInfo :type Struct%20Player%20Info%20Structure))
  ;[1 1 1] Respawn player
  (Default|RespawnPlayer (Variables|Default|GetGameModeRef) self PlayerInfo))

(event Custom|DestroySessionForPlayer
  ;[1 1 1] Destroy session for player
  (Default|CallDestroySession (.AsBP%20Game%20Instance (Utilities|Casting|CastToBP_GameInstance (Game|GetGameInstance))) self))

(event Custom|PlayerDead
  ;[1 1 1] Destroy player pawn and respawn
  (bind _output_get (Variables|PlayerStates|SetHealth 1.0))
  (Default|UpdateStatus (Variables|Default|GetHudRef) _output_get)
  (CallFunction|CallRespawnPlayer))

(event Custom|UpdateComSysPosition
  (params (Index :type Integer) (TaggedActor :type Actor%20Object%20Reference))
  ;[1 1 1] Communication system events
  ;;[1 1 1] Update ComSys position
  (Default|SetComSysPos (Variables|Default|GetHudRef) Index (.ScreenPosition (Class|GameplayStatics|ProjectWorldtoScreen self (Transformation|GetActorLocation TaggedActor) true))))

(event Custom|TakeDamage
  ;[1 1 1] Take damage
  (if (Variables|PlayerStates|GetCanTakeDamage)
    (bind _output_get (Variables|Default|Sethealth (- (Variables|Default|Gethealth) 0.1)))
    (Default|UpdateStatus (Variables|Default|GetHudRef) _output_get)
    (if (<= (Variables|Default|Gethealth) 0.01)
      (CallFunction|PlayerDead)
      (else
        (Variables|PlayerStates|SetCanTakeDamage false)
        (Utilities|FlowControl|Delay 1.0)
        (Variables|PlayerStates|SetCanTakeDamage true)))))

(event Custom|CallAttackPlayerChar
  (params (Team :type Enum_PlayerTeam%20Enum) (Player%20Character :type Character%20Object%20Reference))
  ;[1 1 1] Attack
  (switch Utilities|FlowControl|Switch|SwitchonEnum_PlayerTeam Team
    (:NewEnumerator0
      (bind _asbp_character_red (Utilities|Casting|CastToBP_CharacterRed Player%20Character))
      (Default|Attack _asbp_character_red))
    (:NewEnumerator1
      (bind _asbp_character_green (Utilities|Casting|CastToBP_CharacterGreen Player%20Character))
      (Default|Attack _asbp_character_green))))

(event Custom|CallRespawnPlayer
  ;[1 1 1] Respawn player
  (CallFunction|PlayerRespawnServerLink (Variables|PlayerData|GetPlayerInfo)))

(event Custom|SendComSysUpdateToServer
  (params (State :type Enum_ComSysState%20Enum) (Actor :type Actor%20Object%20Reference) (Team :type Enum_PlayerTeam%20Enum) (Index :type Integer))
  ;[1 1 1] Communication system events
  (Default|UpdateComSysUnit (Variables|Default|GetGameModeRef) Team Index State Actor))

(event Custom|ToggleRunPlayerChar
  (params (Team :type Enum_PlayerTeam%20Enum) (PlayerCharacter :type Character%20Object%20Reference) (ToRun :type Boolean))
  ;[1 1 1] Run
  (switch Utilities|FlowControl|Switch|SwitchonEnum_PlayerTeam Team
    (:NewEnumerator0
      (bind _asbp_character_red (Utilities|Casting|CastToBP_CharacterRed PlayerCharacter))
      (if ToRun
        (Default|RunStart _asbp_character_red)
        (else
          (Default|RunStop _asbp_character_red))))
    (:NewEnumerator1
      (bind _asbp_character_green (Utilities|Casting|CastToBP_CharacterGreen PlayerCharacter))
      (if ToRun
        (Default|RunStart _asbp_character_green)
        (else
          (Default|RunStop _asbp_character_green))))))

(event Custom|UpdateComSysState
  (params (Index :type Integer) (State :type Enum_ComSysState%20Enum))
  ;[1 1 1] Communication system events
  ;;[1 1 1] Update ComSys state
  (Default|SetComSysState (Variables|Default|GetHudRef) Index State))

(event Custom|UpdateTeamBars
  (params (Red :type Float%20%28single-precision%29) (Green :type Float%20%28single-precision%29))
  ;[1 1 1] Update team bars
  (Default|UpdateTeamBars (Variables|Default|GetHudRef) Red Green))

(event Custom|SetComSysIndexInClient
  (params (Index :type Integer))
  ;[1 1 1] Server stuff
  (Variables|ComSys|SetComSysIndex Index))

(event Custom|MoveForwardPlayerChar
  (params (Team :type Enum_PlayerTeam%20Enum) (PlayerCharacter :type Character%20Object%20Reference) (AxisValue :type Float%20%28single-precision%29))
  (switch Utilities|FlowControl|Switch|SwitchonEnum_PlayerTeam Team
    (:NewEnumerator0
      (bind _asbp_character_red (Utilities|Casting|CastToBP_CharacterRed PlayerCharacter))
      (Default|MovementForward _asbp_character_red AxisValue))
    (:NewEnumerator1
      (bind _asbp_character_green (Utilities|Casting|CastToBP_CharacterGreen PlayerCharacter))
      (Default|MovementForward _asbp_character_green AxisValue))))

(event Custom|MoveRightPlayerChar
  (params (Team :type Enum_PlayerTeam%20Enum) (PlayerCharacter :type Character%20Object%20Reference) (AxisValue :type Float%20%28single-precision%29))
  (switch Utilities|FlowControl|Switch|SwitchonEnum_PlayerTeam Team
    (:NewEnumerator0
      (bind _asbp_character_red (Utilities|Casting|CastToBP_CharacterRed PlayerCharacter))
      (Default|MovementRight _asbp_character_red AxisValue))
    (:NewEnumerator1
      (bind _asbp_character_green (Utilities|Casting|CastToBP_CharacterGreen PlayerCharacter))
      (Default|MovementRight _asbp_character_green AxisValue))))

(event Input|ActionEvents|InputActionComSysAttack
  (params (Key :type Key%20Structure :default "AnyKey"))
  ;[1 1 1] Communication system events
  ;;[1 1 1] ComSys action attack
  (:Pressed
    (bind _state (Utilities|GetComsysState))
    (if (Utilities|Enum|Equal(Enum) _state "NewEnumerator0")
      (Utilities|UpdateComSysinGameMode "NewEnumerator4")
      (else
        (switch Utilities|FlowControl|Switch|SwitchonEnum_PlayerTeam (.Team (Utilities|Struct|BreakStruct_PlayerInfo (Variables|PlayerData|GetPlayerInfo)))
          (:NewEnumerator0
            (bind (_hitresults _didhitobject) (Utilities|RayTracefromCharacter)
              (:Out
                (if _didhitobject
                  (bind (_found _actor) (CallFunction|SearchforEnemy "NewEnumerator1" _hitresults))
                  (if _found
                    (Utilities|UpdateComSysinGameMode "NewEnumerator0" _actor))))))
          (:NewEnumerator1
            (bind (_hitresults_2 _didhitobject_2) (Utilities|RayTracefromCharacter)
              (:Out
                (if _didhitobject_2
                  (bind (_found_2 _actor_2) (CallFunction|SearchforEnemy "NewEnumerator0" _hitresults_2))
                  (if _found_2
                    (Utilities|UpdateComSysinGameMode "NewEnumerator0" _actor_2)))))))))))

(event Input|ActionEvents|InputActionComSysFollow
  (params (Key :type Key%20Structure :default "AnyKey"))
  ;[1 1 1] Communication system events
  ;;[1 1 1] ComSys action follow
  (:Pressed
    (bind _state (Utilities|GetComsysState))
    (if (Utilities|Enum|Equal(Enum) _state "NewEnumerator2")
      (Utilities|UpdateComSysinGameMode "NewEnumerator4")
      (else
        (Utilities|UpdateComSysinGameMode "NewEnumerator2" (Variables|PlayerData|GetPlayerCharacterRef))))))

(event Input|ActionEvents|InputActionComSysHeal
  (params (Key :type Key%20Structure :default "AnyKey"))
  ;[1 1 1] Communication system events
  ;;[1 1 1] ComSys action heal
  (:Pressed
    (bind _state (Utilities|GetComsysState))
    (if (Utilities|Enum|Equal(Enum) _state "NewEnumerator3")
      (Utilities|UpdateComSysinGameMode "NewEnumerator4")
      (else
        (Utilities|UpdateComSysinGameMode "NewEnumerator3" (Variables|PlayerData|GetPlayerCharacterRef))))))

(event Input|ActionEvents|InputActionRun
  (params (Key :type Key%20Structure :default "AnyKey"))
  (bind _playerinfo (Variables|PlayerData|GetPlayerInfo))
  (bind _playercharacterref (Variables|PlayerData|GetPlayerCharacterRef))
  (bind _team (Utilities|Struct|BreakStruct_PlayerInfo _playerinfo))
  ;[1 1 1] Run
  (:Pressed
    (CallFunction|ToggleRunPlayerChar _team _playercharacterref true))
  (:Released
    (CallFunction|ToggleRunPlayerChar _team _playercharacterref false)))

(event Input|ActionEvents|InputActionComSysDeffend
  (params (Key :type Key%20Structure :default "AnyKey"))
  ;[1 1 1] Communication system events
  ;;[1 1 1] ComSys action deffend
  (:Pressed
    (bind _state (Utilities|GetComsysState))
    (if (Utilities|Enum|Equal(Enum) _state "NewEnumerator1")
      (Utilities|UpdateComSysinGameMode "NewEnumerator4")
      (else
        (bind (_hitresults _didhitobject) (Utilities|RayTracefromCharacter)
          (:Out
            (if _didhitobject
              (bind (_found _actor) (CallFunction|SearchforZone _hitresults))
              (if _found
                (Utilities|UpdateComSysinGameMode "NewEnumerator1" _actor)))))))))

(event Input|ActionEvents|InputActionAttack
  (params (Key :type Key%20Structure :default "AnyKey"))
  ;[1 1 1] Attack
  (:Pressed
    (CallFunction|CallAttackPlayerChar (.Team (Utilities|Struct|BreakStruct_PlayerInfo (Variables|PlayerData|GetPlayerInfo))) (Variables|PlayerData|GetPlayerCharacterRef))))

(fn ConstructionScript
  (bind _asbp_gameplay_gm (Utilities|Casting|CastToBP_GameplayGM (Game|GetGameMode)))
  (Variables|Default|SetGameModeRef _asbp_gameplay_gm))

(fn SearchforEnemy
  (params (EnemyTeam :type Enum_PlayerTeam%20Enum) (HitResults :type Array%20of%20Hit%20Result%20Structures))
  (switch Utilities|FlowControl|Switch|SwitchonEnum_PlayerTeam EnemyTeam
    (:NewEnumerator2
      _)
    (:NewEnumerator0
      (bind _array_element (Utilities|Array|ForEachLoopwithBreak HitResults :!label _label)
        (:LoopBody
          (bind _asbp_character_red (Utilities|Casting|CastToBP_CharacterRed (|GetHitActors _array_element)))
          (LocalVariables|SetEnemyFound true)
          (LocalVariables|SetEnemyActor _asbp_character_red)
          (goto _label Break))
        (:Completed
          _)))
    (:NewEnumerator1
      (bind _array_element_2 (Utilities|Array|ForEachLoopwithBreak HitResults :!label _label_2)
        (:LoopBody
          (bind _asbp_character_green (Utilities|Casting|CastToBP_CharacterGreen (|GetHitActors_2 _array_element_2)))
          (LocalVariables|SetEnemyFound true)
          (LocalVariables|SetEnemyActor _asbp_character_green)
          (goto _label_2 Break))
        (:Completed
          _))))
  (return (LocalVariables|GetEnemyFound) (LocalVariables|GetEnemyActor)))

(fn SearchforZone
  (params (HitResults :type Array%20of%20Hit%20Result%20Structures))
  (bind _array_element (Utilities|Array|ForEachLoopwithBreak HitResults :!label _label)
    (:LoopBody
      (bind _aspb_zone (Utilities|Casting|CastToPB_Zone (|GetHitActors _array_element)))
      (LocalVariables|SetZoneFound true)
      (LocalVariables|SetZoneActor _aspb_zone)
      (goto _label Break))
    (:Completed
      (return (LocalVariables|GetZoneFound) (LocalVariables|GetZoneActor)))))

(fn OnRepPlayerInfo)