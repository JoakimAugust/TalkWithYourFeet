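; BP_TravelMapGM is the game mode for the travel map, a pre-match staging level that gathers players before server travel to GameMap.
; It reads MaxPlayers from BP_GameInstance and collects controllers on PostLogin, running each one's initial setup.
; When the count matches, it shows the ready state on the first player's loading screen and alternates red/green team and character assignments through UpdateInfo.
; StartGame performs the server travel only once the game is startable.
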(event Custom|SetPlayerInfo
  ;[1 1 1] Set player character, team and name
  (Networking|SwitchHasAuthority
    (:Authority
      (for _array_element (Variables|Default|GetPlayerControllers)
        (bind _asbp_travel_map_pc (Utilities|Casting|CastToBP_TravelMapPC _array_element))
        (if (Variables|Default|GetGreenTeam)
          (Variables|Default|SetGreenTeam false)
          (Default|UpdateInfo _asbp_travel_map_pc (Utilities|Struct|MakeStruct_PlayerInfo (.Name (Utilities|Struct|BreakStruct_PlayerInfo (Variables|/Game/Blueprints/TravelMap/BP_TravelMapPC.BP_TravelMapPC_C|GetPlayerInfo _asbp_travel_map_pc))) "/Game/Blueprints/Gameplay/Characters/BP_CharacterGreen.BP_CharacterGreen_C" "NewEnumerator1"))
          (else
            (Variables|Default|SetGreenTeam true)
            (Default|UpdateInfo _asbp_travel_map_pc (Utilities|Struct|MakeStruct_PlayerInfo (.Name (Utilities|Struct|BreakStruct_PlayerInfo (Variables|/Game/Blueprints/TravelMap/BP_TravelMapPC.BP_TravelMapPC_C|GetPlayerInfo _asbp_travel_map_pc))) "/Game/Blueprints/Gameplay/Characters/BP_CharacterRed.BP_CharacterRed_C" "NewEnumerator0"))))))))

(event Custom|StartGame
  ;[1 1 1] Start game
  (if (Variables|Default|GetGameStartable)
    (Development|ExecuteConsoleCommand "servertravel  /Game/Maps/GameMap" (Game|GetPlayerController 0))))

(event EventPostLogin
  (params (NewPlayer :type Player%20Controller%20Object%20Reference))
  (bind _playercontrollers (Variables|Default|GetPlayerControllers))
  ;[1 1 1] On post login setup
  (Networking|SwitchHasAuthority
    (:Authority
      (Utilities|Array|Add _playercontrollers NewPlayer)
      (Variables|Default|SetGameStartable (== (Variables|Default|GetMaxPlayers) (Utilities|Array|Length _playercontrollers)))
      (bind _asbp_travel_map_pc (Utilities|Casting|CastToBP_TravelMapPC NewPlayer))
      (Default|InitialSetup _asbp_travel_map_pc)
      (if (Variables|Default|GetGameStartable)
        (|SetServerLoadingScreen)
        (CallFunction|SetPlayerInfo)))))

(fn ConstructionScript
  (Networking|SwitchHasAuthority
    (:Authority
      (bind _asbp_game_instance (Utilities|Casting|CastToBP_GameInstance (Game|GetGameInstance)))
      (Variables|Default|SetMaxPlayers (Variables|/Game/Blueprints/General/BP_GameInstance.BP_GameInstance_C|GetMaxPlayers _asbp_game_instance)))))