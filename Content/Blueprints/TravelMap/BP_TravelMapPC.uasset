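; BP_TravelMapPC is, by its name, the player controller for the travel map, handling player info and session cleanup.
; The construction script caches a reference to BP_GameInstance.
; InitialSetup shows the loading screen, reads PlayerInfo from the game instance and passes it to UpdateInfo, which stores it locally and writes it back.
; EndPlay destroys the session.
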(event Custom|UpdateInfo
  (params (PlayerInfo :type Struct%20Player%20Info%20Structure))
  (bind _gameinstanceref (Variables|Default|GetGameInstanceRef))
  ;[1 1 1] Update player
  (Variables|Default|SetPlayerInfo PlayerInfo)
  (Utilities|IsValid _gameinstanceref
    (:Is%20Valid
      (Variables|/Game/Blueprints/General/BP_GameInstance.BP_GameInstance_C|SetPlayerInfo _gameinstanceref (Variables|Default|GetPlayerInfo)))))

(event Custom|InitialSetup
  (bind _gameinstanceref (Variables|Default|GetGameInstanceRef))
  ;[1 1 1] Initial setup
  (Default|ShowLoadingScreen _gameinstanceref)
  (Utilities|IsValid _gameinstanceref
    (:Is%20Valid
      (Variables|Default|SetPlayerInfo (Variables|/Game/Blueprints/General/BP_GameInstance.BP_GameInstance_C|GetPlayerInfo _gameinstanceref))
      (CallFunction|UpdateInfo (Variables|Default|GetPlayerInfo)))))

(event EventEndPlay
  (params (EndPlayReason :type EEndPlayReason%20Enum :default "Destroyed"))
  ;[1 1 1] End play
  (|DestroySession self))

(fn ConstructionScript
  (bind _asbp_game_instance (Utilities|Casting|CastToBP_GameInstance (Game|GetGameInstance)))
  (Variables|Default|SetGameInstanceRef _asbp_game_instance))